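; BP_EnemyBase is an enemy character Blueprint that sets up its ability system and weapon on BeginPlay.
; It applies the default attributes effect to itself, then finds a BP_WeaponBase actor already in the level with GetActorOfClass.
; EquipWeapon stores that weapon in the combat component and calls its OnEquipped.
; A separate sequence branch grants and activates GA_Stagger once after a short delay.
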(event `self.ReceiveBeginPlay`
  (`|ExecutionSequence`
    (:`then_0`
      (`AbilitySystemComponent.BP_ApplyGameplayEffectToSelf` :`self` (`AbilitySystemBlueprintLibrary.GetAbilitySystemComponent` null) :`GameplayEffectClass` "/Game/MyContent/AI/GameplayEffects/GE_DefaultAttributes.GE_DefaultAttributes_C")
      (bind _returnvalue (`GameplayStatics.GetActorOfClass` "/Game/MyContent/Weapon/Actor/BP_WeaponBase.BP_WeaponBase_C"))
      (`self.EquipWeapon` _returnvalue))
    (:`then_1`
      (`KismetSystemLibrary.Delay` 3.0)
      (`AbilitySystemComponent.K2_GiveAbilityAndActivateOnce` (`self.AbilitySystemComponent`) "/Game/MyContent/AI/GameplayAbility/GA_Stagger.GA_Stagger_C" 0 -1))))

(event `self.ReceiveTick`
  (params (DeltaSeconds :type "Float (single-precision)")))

(fn `EquipWeapon`
  (params (`New Weapon` :type "/Game/MyContent/Weapon/Actor/BP_WeaponBase Object Reference"))
  (bind _output_get (set `/Game/MyContent/AI/Component/BP_CombatComponent.CurrentWeapon` `New Weapon` (`self.BP_CombatComponent`)))
  (`/Game/MyContent/Weapon/Actor/BP_WeaponBase.OnEquipped` _output_get self))

(fn `UserConstructionScript`)