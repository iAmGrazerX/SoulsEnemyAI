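; GA_LightAttack is a Gameplay Ability that runs an enemy's light attack on a BP_EnemyBase avatar.
; When stamina is zero or above, it manually applies the GE_Cost_LightAttack effect and plays the AM_ComboAttack montage; otherwise it ends.
; Montage completion sends Ability.Attack.Finished to the enemy's StateTree AI component and ends the ability; interruption is not handled.
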(event `self.K2_ActivateAbility`
  (bind _asbp_enemy_base (cast `/Game/MyContent/Character/BP_EnemyBase` (`self.GetAvatarActorFromActorInfo`)))
  (if (>= (`EnemyCharacterBase.GetCurrentStamina` _asbp_enemy_base) 0.0)
    (`self.BP_ApplyGameplayEffectToOwner` "/Game/MyContent/AI/GAS/GameplayEffects/GE_Cost_LightAttack.GE_Cost_LightAttack_C")
    (`|PlayMontage` (`Character.Mesh` _asbp_enemy_base) "/Game/Variant_Combat/Anims/AM_ComboAttack.AM_ComboAttack"
      (:`then`
        (`KismetSystemLibrary.PrintString` "GA_LightAttack : Activated" true true (struct :`R` 0.160456 :`G` 0.046975 :`B` 1.0 :`A` 1.0)))
      (:`OnCompleted`
        (`StateTreeComponent.SendStateTreeEvent` (`/Game/MyContent/Character/BP_EnemyBase.Enemy StateTreeAIComponent` _asbp_enemy_base) (make `StateTreeEvent` (struct :`TagName` "Ability.Attack.Finished")))
        (`self.K2_EndAbility`)))
    (else
      (`KismetSystemLibrary.PrintString` "GA_LightAttack : Failed" true true (struct :`R` 0.160456 :`G` 0.046975 :`B` 1.0 :`A` 1.0))
      (`self.K2_EndAbility`))))

(event `self.K2_OnEndAbility`
  (params (bWasCancelled :type Boolean)))