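; GA_HeavyAttack is a Gameplay Ability that performs a heavy attack for EnemyCharacterBase avatars.
; If stamina is at least zero, it applies GE_Cost_LightAttack to the owner as its cost and plays AM_ComboAttack on the mesh.
; It ends on montage completion or a failed stamina check, but not on montage interruption or a failed cast.
; Debug prints report activation, failure and end.
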(event `self.K2_ActivateAbility`
  (bind _asenemy_character_base (cast `EnemyCharacterBase` (`self.GetAvatarActorFromActorInfo`)))
  (if (>= (`EnemyCharacterBase.GetCurrentStamina` _asenemy_character_base) 0.0)
    (`self.BP_ApplyGameplayEffectToOwner` "/Game/MyContent/AI/GAS/GameplayEffects/GE_Cost_LightAttack.GE_Cost_LightAttack_C")
    (`|PlayMontage` (`Character.Mesh` _asenemy_character_base) "/Game/Variant_Combat/Anims/AM_ComboAttack.AM_ComboAttack"
      (:`then`
        (`KismetSystemLibrary.PrintString` "GA_HeavyAttack : Activated" true true (struct :`R` 0.160456 :`G` 0.046975 :`B` 1.0 :`A` 1.0)))
      (:`OnCompleted`
        (`self.K2_EndAbility`)))
    (else
      (`KismetSystemLibrary.PrintString` "GA_HeavyAttack : Failed" true true (struct :`R` 0.160456 :`G` 0.046975 :`B` 1.0 :`A` 1.0))
      (`self.K2_EndAbility`))))

(event `self.K2_OnEndAbility`
  (params (bWasCancelled :type Boolean))
  (`KismetSystemLibrary.PrintString` "GA_HeavyAttack : Ended" true true (struct :`R` 0.160456 :`G` 0.046975 :`B` 1.0 :`A` 1.0)))