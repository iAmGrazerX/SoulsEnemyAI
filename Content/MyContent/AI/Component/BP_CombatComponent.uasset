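; AI combat component that makes its owner chase and attack the player, targeted at BeginPlay.
; A looping timer classifies target distance against the current weapon's combat profile as too close, in range or too far.
; Tick approaches when too far and attacks in range, activating the GAS ability returned by the weapon for a close-range intent.
; Timers handle attack recovery and stagger; stagger stops movement and blocks attacks, but not renewed approach.
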(event `self.ReceiveBeginPlay`
  (set `self.CurrentTarget` (`GameplayStatics.GetPlayerCharacter` 0))
  (`KismetSystemLibrary.K2_SetTimer` null "EvaluateDistance" 1.0 true))

(event `self.ReceiveTick`
  (params (DeltaSeconds :type "Float (single-precision)"))
  (`|ExecutionSequence`
    (:`then_0`
      (if (`|EnumEquality` (`self.CurrentRangeState`) "NewEnumerator2")
        (`self.ApproachTarget`)))
    (:`then_1`
      (if (`|EnumEquality` (`self.CurrentRangeState`) "NewEnumerator1")
        (`self.Attack`)))))

(fn `ApproachTarget`
  (`AIController.MoveToActor` (`AIBlueprintHelperLibrary.GetAIController` (`self.GetOwner`)) (`self.CurrentTarget`) -1.0 true true true null true)
  (set `self.CurrentCombatState` "NewEnumerator2"))

(fn `Attack`
  (bind (_currentcombatprofile_mincombatrange _currentcombatprofile_idealcombatrange _currentcombatprofile_maxcombatrange _currentcombatprofile_recoveryduration) (break `CombatProfile` (`self.CurrentCombatProfile`)))
  (if (and (`KismetSystemLibrary.IsValid` (`self.CurrentTarget`)) (!= (`self.IsRecovering`) true) (`|EnumInequality` (`self.CurrentCombatState`) "NewEnumerator4"))
    (set `self.IsRecovering` true)
    (set `self.CurrentCombatState` "NewEnumerator2")
    (bind _ability_class (`/Game/MyContent/Weapon/Actor/BP_WeaponBase.Request Intent` (`self.CurrentWeapon`) "CloseRangeAttack"))
    (`AbilitySystemComponent.TryActivateAbilityByClass` (`AbilitySystemBlueprintLibrary.GetAbilitySystemComponent` (`self.GetOwner`)) _ability_class true)
    (bind _returnvalue (`KismetSystemLibrary.K2_SetTimer` null "Reset Recovery" _currentcombatprofile_recoveryduration))
    (set `self.RecoveryTimerHandle` _returnvalue)))

(fn `EnterStagger`
  (params (Duration :type "Float (double-precision)"))
  (set `self.CurrentCombatState` "NewEnumerator4")
  (set `self.IsRecovering` false)
  (`Controller.StopMovement` (`AIBlueprintHelperLibrary.GetAIController` (`self.GetOwner`)))
  (`KismetSystemLibrary.K2_SetTimer` null "ExitStagger" Duration))

(fn `EvaluateDistance`
  (bind (_mincombatrange _idealcombatrange _maxcombatrange) (break `CombatProfile` (`self.CurrentCombatProfile`)))
  (bind _currentdistance (`self.GetDistanceToTarget`))
  (if (< _currentdistance _mincombatrange)
    (set `self.CurrentRangeState` "NewEnumerator0")
    (elif (> _currentdistance _maxcombatrange)
      (set `self.CurrentRangeState` "NewEnumerator2")
      (else
        (set `self.CurrentRangeState` "NewEnumerator1"))))
  (`KismetSystemLibrary.PrintString` (`|GetEnumeratorNameAsString` (`self.CurrentRangeState`)))
  (`KismetSystemLibrary.PrintString` (`KismetStringLibrary.Conv_DoubleToString` _currentdistance)))

(fn `ExitStagger`
  (set `self.CurrentCombatState` "NewEnumerator0"))

(fn `GetDistanceToTarget`
  (returns (CurrentDistance :type "Float (double-precision)"))
  (return (`KismetMathLibrary.Vector_Distance` (`Actor.K2_GetActorLocation` (`self.GetOwner`)) (`Actor.K2_GetActorLocation` (`self.CurrentTarget`)))))

(fn `IsTooClose`
  (returns (TooClose :type Boolean))
  (return (`|EnumEquality` (`self.CurrentRangeState`) "NewEnumerator0")))

(fn `IsTooFar`
  (returns (TooFar :type Boolean))
  (return (`|EnumEquality` (`self.CurrentRangeState`) "NewEnumerator2")))

(fn `Reset Recovery`
  (set `self.IsRecovering` false)
  (`KismetSystemLibrary.K2_ClearAndInvalidateTimerHandle` (`self.RecoveryTimerHandle`))
  (set `self.CurrentCombatState` "NewEnumerator0")
  (`KismetSystemLibrary.PrintString` "Recovered"))

(fn `SetWeapon`
  (params (Weapon :type "/Game/MyContent/Weapon/Actor/BP_WeaponBase Object Reference"))
  (bind _output_get (set `self.CurrentWeapon` Weapon))
  (set `self.CurrentCombatProfile` (`/Game/MyContent/Weapon/Actor/BP_WeaponBase.CombatProfile` _output_get)))